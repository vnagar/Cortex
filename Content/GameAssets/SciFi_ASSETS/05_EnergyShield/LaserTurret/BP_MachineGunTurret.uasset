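; BP_MachineGunTurret is a machine gun turret that activates and plays its firing animation when an actor overlaps it.
; Begin overlap plays the activate animation, then after a one-second delay loops the fire animation and sets IsFiring; end overlap clears it and plays deactivation.
; A timeline fades the lights' emissive intensity through a Material Parameter Collection, reversing on exit.
; FollowPlayerPosition is an empty stub.
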(event Collision|EventActorBeginOverlap
  (params (OtherActor :type Actor%20Object%20Reference))
  (bind _sk_machinegunturret_01 (Variables|Default|GetSK_MachineGunTurret_01))
  (Utilities|FlowControl|Sequence
    (:then_0
      (Components|Animation|PlayAnimation _sk_machinegunturret_01 "/Game/GameAssets/SciFi_ASSETS/05_EnergyShield/LaserTurret/Animations/A_MGT_Activate.A_MGT_Activate" false)
      (Utilities|FlowControl|Delay 1.0)
      (Components|Animation|PlayAnimation _sk_machinegunturret_01 "/Game/GameAssets/SciFi_ASSETS/05_EnergyShield/LaserTurret/Animations/AM_MGT_Fire.AM_MGT_Fire" true)
      (Variables|Default|SetIs%20Firing true))
    (:then_1
      (bind _emissive_intensity (Timeline|Activate%20Lights Play)
        (:Update
          (Rendering|Material|SetScalarParameterValue "/Game/GameAssets/SciFi_ASSETS/05_EnergyShield/LaserTurret/Materials/MPC_TurretLights.MPC_TurretLights" "Emissive Intensity" (* _emissive_intensity 15.0) :!class /Script/Engine.KismetMaterialLibrary))))))

(event Collision|EventActorEndOverlap
  (params (OtherActor :type Actor%20Object%20Reference))
  (bind _sk_machinegunturret_01 (Variables|Default|GetSK_MachineGunTurret_01))
  (Variables|Default|SetIs%20Firing false)
  (Utilities|FlowControl|Sequence
    (:then_0
      (Audio|Components|Audio|Stop _sk_machinegunturret_01)
      (Components|Animation|PlayAnimation _sk_machinegunturret_01 "/Game/GameAssets/SciFi_ASSETS/05_EnergyShield/LaserTurret/Animations/A_MGT_Deactivate.A_MGT_Deactivate" false))
    (:then_1
      (bind _emissive_intensity (Timeline|Activate%20Lights Reverse)
        (:Update
          (Rendering|Material|SetScalarParameterValue "/Game/GameAssets/SciFi_ASSETS/05_EnergyShield/LaserTurret/Materials/MPC_TurretLights.MPC_TurretLights" "Emissive Intensity" (* _emissive_intensity 15.0) :!class /Script/Engine.KismetMaterialLibrary))))))

(fn ConstructionScript)

(fn FollowPlayerPosition)