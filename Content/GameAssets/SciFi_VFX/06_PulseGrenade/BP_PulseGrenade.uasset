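; Pulse grenade Blueprint in the sci-fi VFX set, whose only logic is bounce audio.
; Capsule hits add an audio component through a DoOnce gate, which reopens after a short delay to debounce repeated contacts.
; A cascade of DoOnce nodes on staggered delays resets each preceding gate, with the last never reset, so only a handful of bounces make sound.
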(event OnComponentHit(Capsule)
  (params (HitComponent :type Primitive%20Component%20Object%20Reference) (OtherActor :type Actor%20Object%20Reference) (OtherComp :type Primitive%20Component%20Object%20Reference) (NormalImpulse :type Vector :default "0, 0, 0") (Hit :type Hit%20Result%20Structure%20%28by%20ref%29))
  ;[1 0 0.4453] BOUNCE AUDIO
  (Utilities|FlowControl|DoOnce false :!label _label
    (:Completed
      (Utilities|FlowControl|Sequence
        (:then_0
          (AddComponent|AddAudioComponent false))
        (:then_1
          (Utilities|FlowControl|Delay 0.1)
          (Utilities|FlowControl|DoOnce false :!label _label_2
            (:Completed
              (goto _label Reset))))
        (:then_2
          (Utilities|FlowControl|Delay 0.15)
          (Utilities|FlowControl|DoOnce false :!label _label_3
            (:Completed
              (goto _label_2 Reset))))
        (:then_3
          (Utilities|FlowControl|Delay 0.2)
          (Utilities|FlowControl|DoOnce false :!label _label_4
            (:Completed
              (goto _label_3 Reset))))
        (:then_4
          (Utilities|FlowControl|Delay 0.25)
          (Utilities|FlowControl|DoOnce false
            (:Completed
              (goto _label_4 Reset))))))))

(event EventBeginPlay)

(fn ConstructionScript)